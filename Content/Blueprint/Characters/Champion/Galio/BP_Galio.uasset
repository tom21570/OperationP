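; Galio champion Blueprint that spawns a damage cube on its mesh after repeated CreateField calls.
; Each CreateField call increments a spawn counter and compares it to DestroyMargin.
; Once the counter reaches that margin, every call spawns a BP_CubeDamage at ChaosDamageSocket and snaps it to that socket, keeping world scale.
; The counter never resets here, and the construction script is empty.
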(event EventCreateField
  (bind _result (Math|Float|IncrementFloat (Variables|Default|GetSpawnedNum))
    (:%20%20
      (Variables|Default|SetSpawnedNum _result)
      (if (>= (Variables|Default|GetSpawnedNum) (Variables|Default|GetDestroyMargin))
        (bind _returnvalue (Game|SpawnActorfromClass "/Game/Blueprint/Chaos/Destruction/BP_CubeDamage.BP_CubeDamage_C" (Transformation|GetSocketTransform (Variables|Character|GetMesh) "ChaosDamageSocket" "RTS_World") "Undefined" "MultiplyWithRoot" 0 0))
        (Transformation|AttachComponentToComponent _returnvalue (Variables|Character|GetMesh) "ChaosDamageSocket" "SnapToTarget" "SnapToTarget" "KeepWorld" true)))))

(fn ConstructionScript)