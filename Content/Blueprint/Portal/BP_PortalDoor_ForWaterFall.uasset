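; Portal door Blueprint, named for a waterfall, that swings open, releases a flood and knocks the player into ragdoll.
; OpenDoor plays a timeline that rotates the door yaw up to 120 degrees.
; Delays on the timeline's update pin activate Flood, then later enable physics on the BP_Avidd pawn's mesh.
; The ragdoll push derives from the player's offset from the door, with Y zeroed and Z inverted.
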(event Custom|OpenDoor
  (bind _새_트랙_0 (Timeline|타임라인 PlayFromStart)
    (:Update
      (Transformation|SetRelativeRotation (Variables|Default|GetDoor) (Math|Rotator|MakeRotator 0.0 0.0 (Math|Float|Lerp 0.0 1.2e+02 _새_트랙_0)) false false)
      (Utilities|FlowControl|Sequence
        (:then_0
          (Utilities|FlowControl|Delay 0.4)
          (Components|Activation|Activate (Variables|Default|GetFlood) false))
        (:then_1
          (Utilities|FlowControl|Delay 0.8)
          (bind _asbp_avidd (Utilities|Casting|CastToBP_Avidd (Game|Player|GetPlayerPawn 0)))
          (Physics|SetSimulatePhysics (Variables|/Script/Engine.Character|GetMesh _asbp_avidd) true)
          (Class|SkeletalMeshComponent|AddForcetoAllBodiesBelow (Variables|/Script/Engine.Character|GetMesh _asbp_avidd) (* (- (Transformation|GetActorLocation _asbp_avidd) (Transformation|GetActorLocation)) "500.000000,0.000000,-500.000000") "None" true true))))))

(event EventBeginPlay)

(event Collision|EventActorBeginOverlap
  (params (OtherActor :type Actor%20Object%20Reference)))

(event EventTick
  (params (DeltaSeconds :type Float%20%28single-precision%29)))

(fn ConstructionScript)