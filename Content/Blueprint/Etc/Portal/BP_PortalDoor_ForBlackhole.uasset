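; BP_PortalDoor_ForBlackhole is a portal door that swings open and drags the player BP_Avidd in like a black hole.
; OpenDoor enables the Box trigger and runs a timeline rotating the door.
; Timeline updates feed a delay, then ragdoll the player and apply force from the Sphere's relative location minus the player's world location.
; When the player's DoorInteractingCollision overlaps the Box, body and head meshes are hidden and a debug string prints.
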(event OnComponentBeginOverlap(Box)
  (params (OverlappedComponent :type Primitive%20Component%20Object%20Reference) (OtherActor :type Actor%20Object%20Reference) (OtherComp :type Primitive%20Component%20Object%20Reference) (OtherBodyIndex :type Integer) (bFromSweep :type Boolean) (SweepResult :type Hit%20Result%20Structure%20%28by%20ref%29))
  (bind _asbp_avidd (Utilities|Casting|CastToBP_Avidd (Game|Player|GetPlayerPawn 0)))
  (if (== (Variables|/Game/Blueprint/Characters/OriginalCharacter/Avidd/BP_Avidd.BP_Avidd_C|GetDoorInteractingCollision _asbp_avidd) OtherComp)
    (Rendering|SetVisibility (Variables|/Script/Engine.Character|GetMesh _asbp_avidd) false false)
    (Development|PrintString "Hello")))

(event Custom|OpenDoor
  (Collision|SetCollisionEnabled (Variables|Default|GetBox) "QueryOnly")
  (bind _새_트랙_0 (Timeline|타임라인 PlayFromStart)
    (:Update
      (Transformation|SetRelativeRotation (Variables|Default|GetDoor) (Math|Rotator|MakeRotator 0.0 0.0 (Math|Float|Lerp 0.0 -1.2e+02 _새_트랙_0)) false false)
      (Utilities|FlowControl|Delay 1.0)
      (bind _asbp_avidd (Utilities|Casting|CastToBP_Avidd (Game|Player|GetPlayerPawn 0)))
      (Physics|SetSimulatePhysics (Variables|/Script/Engine.Character|GetMesh _asbp_avidd) true)
      (Class|SkeletalMeshComponent|AddForcetoAllBodiesBelow (Variables|/Script/Engine.Character|GetMesh _asbp_avidd) (* (- (Variables|/Script/Engine.SceneComponent|GetRelativeLocation (Variables|Default|GetSphere)) (Transformation|GetActorLocation _asbp_avidd)) 3e+01) "None" false true))))

(event EventBeginPlay
  (Collision|SetCollisionEnabled (Variables|Default|GetBox) "NoCollision"))

(event Collision|EventActorBeginOverlap
  (params (OtherActor :type Actor%20Object%20Reference)))

(event EventTick
  (params (DeltaSeconds :type Float%20%28single-precision%29)))

(fn ConstructionScript)