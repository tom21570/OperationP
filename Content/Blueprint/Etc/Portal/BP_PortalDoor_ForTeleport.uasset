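; Teleport portal door that sends the player to the DoraemonEgypt level.
; The trigger sphere starts with collision disabled, so the portal is inactive until OpenDoor is called.
; OpenDoor plays a timeline that swings the door open around yaw and enables query collision on the sphere during its updates.
; When the player pawn overlaps the sphere, it opens the level and then hides the pre-teleport plane.
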(event OnComponentBeginOverlap(Sphere)
  (params (OverlappedComponent :type Primitive%20Component%20Object%20Reference) (OtherActor :type Actor%20Object%20Reference) (OtherComp :type Primitive%20Component%20Object%20Reference) (OtherBodyIndex :type Integer) (bFromSweep :type Boolean) (SweepResult :type Hit%20Result%20Structure%20%28by%20ref%29))
  (if (== OtherActor (Game|Player|GetPlayerPawn 0))
    (Game|OpenLevel(byName) "DoraemonEgypt")
    (Rendering|SetVisibility (Variables|Default|GetPlane_BeforeTeleport) false false)))

(event Custom|OpenDoor
  (bind _새_트랙_0 (Timeline|타임라인 Play)
    (:Update
      (Transformation|SetRelativeRotation (Variables|Default|GetDoor) (Math|Rotator|MakeRotator 0.0 0.0 (Math|Float|Lerp 0.0 -1.2e+02 _새_트랙_0)) false false)
      (Collision|SetCollisionEnabled (Variables|Default|GetSphere) "QueryOnly"))))

(event EventBeginPlay
  (Collision|SetCollisionEnabled (Variables|Default|GetSphere) "NoCollision"))

(event Collision|EventActorBeginOverlap
  (params (OtherActor :type Actor%20Object%20Reference)))

(event EventTick
  (params (DeltaSeconds :type Float%20%28single-precision%29)))

(fn ConstructionScript)